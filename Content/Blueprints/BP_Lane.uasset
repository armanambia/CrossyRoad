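; One lane tile in an endlessly spawned, Crossy Road-style track of grass, road, river and railroad lanes.
; SetLaneBegin picks the mesh from LaneSpawner's lane type, spawns a grass, river or vehicle actor (car or train), then counts down the spawner's run of that type.
; When active, its trigger makes LaneSpawner add a lane on player overlap and cull the oldest past the limit.
; EndPlay destroys the lane's spawned actor.
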(event `self.TriggerZone.OnComponentBeginOverlap`
  (params (OverlappedComponent :type "PrimitiveComponent Object Reference") (OtherActor :type "Actor Object Reference") (OtherComp :type "PrimitiveComponent Object Reference") (OtherBodyIndex :type Integer) (bFromSweep :type Boolean) (SweepResult :type "HitResult Structure (by ref)"))
  (bind _lanespawner (`self.LaneSpawner`))
  (bind _lanespawner_2 (`self.LaneSpawner`))
  (bind _alllanes (`/Game/Blueprints/BP_LaneSpawner.allLanes` _lanespawner_2))
  (if (`self.triggerActive`)
    (cast `/Game/Blueprints/BP_MyPlayer` OtherActor)
    (`/Game/Blueprints/BP_LaneSpawner.Spawn Lane at Spawn Point` _lanespawner)
    (if (> (`/Game/Blueprints/BP_LaneSpawner.numLanes` _lanespawner) (`/Game/Blueprints/BP_LaneSpawner.maxLanes` _lanespawner))
      (`self.K2_DestroyActor` (`|GetArrayItem` _alllanes))
      (`KismetArrayLibrary.Array_Remove` _alllanes)
      (bind _result (`/Engine/EditorBlueprintResources/StandardMacros.DecrementInt` (`/Game/Blueprints/BP_LaneSpawner.numLanes` _lanespawner_2))
        (:`  `
          (set `/Game/Blueprints/BP_LaneSpawner.numLanes` _result _lanespawner_2))))))

(event `self.ReceiveEndPlay`
  (params (EndPlayReason :type "EEndPlayReason Enum" :default "Destroyed"))
  (`/Engine/EditorBlueprintResources/StandardMacros.IsValid` (`self.curVehicle`)
    (:`Is Valid`
      (`self.K2_DestroyActor` (`self.curVehicle`)))
    (:`Is Not Valid`
      _))
  (`/Engine/EditorBlueprintResources/StandardMacros.IsValid` (`self.curRiver`)
    (:`Is Valid`
      (`self.K2_DestroyActor` (`self.curRiver`)))
    (:`Is Not Valid`
      _))
  (`/Engine/EditorBlueprintResources/StandardMacros.IsValid` (`self.curGrass`)
    (:`Is Valid`
      (`self.K2_DestroyActor` (`self.curGrass`)))))

(fn `Set Grass Lane`
  (`SceneComponent.K2_AddLocalOffset` (`self.LaneMesh`) (0.0 0.0 -12.0) false false)
  (if (== (`/Game/Blueprints/BP_LaneSpawner.laneTypeCount` (`self.LaneSpawner`)) 2)
    (set `/Game/Blueprints/BP_LaneSpawner.grassHelper` (`KismetMathLibrary.RandomInteger` 2) (`self.LaneSpawner`)))
  (if (== (`/Game/Blueprints/BP_LaneSpawner.grassHelper` (`self.LaneSpawner`)) 0)
    (`StaticMeshComponent.SetStaticMesh` (`self.LaneMesh`) "/Game/Lanes/LightGrass.LightGrass")
    (else
      (`StaticMeshComponent.SetStaticMesh` (`self.LaneMesh`) "/Game/Lanes/DarkGrass.DarkGrass")))
  (bind _returnvalue (`|SpawnActorFromClass` "/Game/Blueprints/BP_Grass.BP_Grass_C" (`KismetMathLibrary.Conv_VectorToTransform` (`SceneComponent.K2_GetComponentLocation` (`self.VehicleSpawn`))) "Undefined" "OverrideRootScale" null null))
  (set `self.curGrass` _returnvalue))

(fn `Set RailRoad Lane`
  (`SceneComponent.K2_AddLocalOffset` (`self.LaneMesh`) (0.0 0.0 -18.75) false false)
  (`StaticMeshComponent.SetStaticMesh` (`self.LaneMesh`) "/Game/Lanes/RailroadFixed.RailroadFixed")
  (`self.Spawn Vehicle`)
  (`/Game/Blueprints/BP_Vehicle.TrainSet` (`self.curVehicle`)))

(fn `Set River Lane`
  (`StaticMeshComponent.SetStaticMesh` (`self.LaneMesh`) "/Game/Lanes/River.River")
  (bind _returnvalue (`|SpawnActorFromClass` "/Game/Blueprints/BP_River.BP_River_C" (`KismetMathLibrary.Conv_VectorToTransform` (`SceneComponent.K2_GetComponentLocation` (`self.VehicleSpawn`))) "Undefined" "OverrideRootScale" null null))
  (bind _output_get (set `self.curRiver` _returnvalue))
  (`/Game/Blueprints/BP_River.RiverSet` _output_get))

(fn `Set Road Lane`
  (if (== (`/Game/Blueprints/BP_LaneSpawner.laneTypeCount` (`self.LaneSpawner`)) 4)
    (`StaticMeshComponent.SetStaticMesh` (`self.LaneMesh`) "/Game/Lanes/UnmarkedRoad.UnmarkedRoad")
    (else
      (`StaticMeshComponent.SetStaticMesh` (`self.LaneMesh`) "/Game/Lanes/MarkedRoad.MarkedRoad")))
  (`self.Spawn Vehicle`)
  (`/Game/Blueprints/BP_Vehicle.RoadSet` (`self.curVehicle`)))

(fn `setLaneBegin`
  (switch `int` (`/Game/Blueprints/BP_LaneSpawner.laneMesh` (`self.LaneSpawner`))
    (:`0`
      (`self.Set Grass Lane`))
    (:`1`
      (`self.Set Road Lane`))
    (:`2`
      (`self.Set River Lane`))
    (:`3`
      (`self.Set RailRoad Lane`)))
  (`self.updateLaneVars`))

(fn `Spawn Vehicle`
  (bind _returnvalue (`|SpawnActorFromClass` "/Game/Blueprints/BP_Vehicle.BP_Vehicle_C" (`KismetMathLibrary.Conv_VectorToTransform` (`SceneComponent.K2_GetComponentLocation` (`self.VehicleSpawn`))) "Undefined" "OverrideRootScale" null null))
  (set `self.curVehicle` _returnvalue)
  (set `/Game/Blueprints/BP_Vehicle.ParentLane` self (`self.curVehicle`)))

(fn `updateLaneVars`
  (`/Engine/EditorBlueprintResources/StandardMacros.DecrementInt` (`/Game/Blueprints/BP_LaneSpawner.laneTypeCount` (`self.LaneSpawner`))
    (:`  `
      (if (<= (`/Game/Blueprints/BP_LaneSpawner.laneTypeCount` (`self.LaneSpawner`)) 0)
        (`/Game/Blueprints/BP_LaneSpawner.resetLaneVars` (`self.LaneSpawner`))))))

(fn `UserConstructionScript`)