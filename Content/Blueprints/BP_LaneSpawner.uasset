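; Spawner for an endless chain of BP_Lane actors that clears and rebuilds the starting run on BeginPlay and game reset.
; The first lane spawns near the player, and each subsequent one spawns at the newest lane's SpawnPoint.
; Once the lane cap is reached, triggers on older lanes are disabled so only front lanes trigger.
; It also holds the current lane mesh type and count, rerolled randomly through ResetLaneVars.
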(event `self.ReceiveBeginPlay`
  (`self.SpawnInitialLanes`))

(fn `prepLane`
  (if (== (`self.laneMesh`) -1)
    (set `self.laneMesh` 0)
    (set `self.laneTypeCount` 2))
  (`/Game/Blueprints/BP_Lane.setLaneBegin` (`self.NewestLane`)))

(fn `resetGame`
  (`GameModeBase.RestartPlayer` (`GameplayStatics.GetGameMode`) null)
  (set `self.numLanes` 0)
  (set `self.laneMesh` 0)
  (set `self.laneTypeCount` 2)
  (set `self.NewestLane` null)
  (`KismetArrayLibrary.Array_Clear` (`self.allLanes`))
  (`self.SpawnInitialLanes`))

(fn `resetLaneVars`
  (bind _output_get (set `self.meshHelper` (select `int` (`KismetMathLibrary.RandomInteger` 4) :`0` 0 :`1` 1 :`2` 2 :`3` 3)))
  (if (== _output_get (`self.laneMesh`))
    (bind _result (`/Engine/EditorBlueprintResources/StandardMacros.DecrementInt` (`self.meshHelper`))
      (:`  `
        (set `self.meshHelper` (`KismetMathLibrary.Abs_Int` _result)))))
  (set `self.laneMesh` (`self.meshHelper`))
  (set `self.laneTypeCount` (select `int` (`self.laneMesh`) :`0` 2 :`1` 4 :`2` 5 :`3` 3)))

(fn `SetTriggers`
  (bind _alllanes (`self.allLanes`))
  (bind _alllanes_2 (`self.allLanes`))
  ;[1 1 1] set triggers if max lanes == num lanes
  (if (> (`self.maxLanes`) (`self.numLanes`))
    _
    (elif (`self.initialTriggers`)
      ;[1 1 1] Set mid lane trigger to false so that only the front lanes trigger
      (set `/Game/Blueprints/BP_Lane.triggerActive` false (`|GetArrayItem` _alllanes (- (/ (`KismetArrayLibrary.Array_Length` _alllanes) 2) 1)))
      (else
        ;[1 1 1] Need to set the first half of lanes to not trigger
        (for (_array_element _array_index) _alllanes_2
          (if (< _array_index (/ (`KismetArrayLibrary.Array_Length` _alllanes_2) 2))
            (set `/Game/Blueprints/BP_Lane.triggerActive` false _array_element)
            (set `self.initialTriggers` true)))))))

(fn `Spawn Lane at Spawn Point`
  (`self.SpawnLane` (`SceneComponent.K2_GetComponentLocation` (`/Game/Blueprints/BP_Lane.SpawnPoint` (`self.NewestLane`)))))

(fn `SpawnInitialLanes`
  (`|ExecutionSequence`
    (:`then_0`
      (bind _outactors (`GameplayStatics.GetAllActorsOfClass` "/Game/Blueprints/BP_Lane.BP_Lane_C"))
      (for _array_element _outactors
        (`self.K2_DestroyActor` _array_element)))
    (:`then_1`
      (for _ (range 5)
        (`/Engine/EditorBlueprintResources/StandardMacros.IsValid` (`self.NewestLane`)
          (:`Is Valid`
            (`self.Spawn Lane at Spawn Point`))
          (:`Is Not Valid`
            (`self.SpawnLane` (`self.K2_GetActorLocation` (`GameplayStatics.GetPlayerPawn` 0)))))))))

(fn `SpawnLane`
  (params (`Spawn Location` :type "Vector Structure"))
  (`self.SetTriggers`)
  (bind _result (`/Engine/EditorBlueprintResources/StandardMacros.IncrementInt` (`self.numLanes`))
    (:`  `
      (set `self.numLanes` _result)
      (bind _returnvalue (`|SpawnActorFromClass` "/Game/Blueprints/BP_Lane.BP_Lane_C" (`KismetMathLibrary.MakeTransform` (`KismetMathLibrary.MakeVector` (+ `Spawn Location_X` 40.0) (`self.Yval`) (`self.Zval`))) "Undefined" "OverrideRootScale" null null))
      (bind _output_get (set `self.NewestLane` _returnvalue))
      (set `/Game/Blueprints/BP_Lane.LaneSpawner` self _output_get)
      (`KismetArrayLibrary.Array_Add` (`self.allLanes`) (`self.NewestLane`))
      (`self.prepLane`))))

(fn `UserConstructionScript`)